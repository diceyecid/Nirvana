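; Closet passcode lock that the player interacts with to open or close a zoomed view of the lock and its passcode UI.
; BeginPlay creates WBP_ClosetPasscodeLock collapsed in the viewport.
; InteractObject finds the overlapping player character, then toggles zoom camera, UI visibility, cursor and Widget component position.
; It always returns false and holds no code-checking logic itself.
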(event EventBeginPlay
  (|CallParentFunction)
  (bind _returnvalue (UserInterface|CreateWidget "/Game/UMG/WBP_ClosetPasscodeLock.WBP_ClosetPasscodeLock_C"))
  (bind _output_get (Variables|Default|SetInteractionUI _returnvalue))
  (UserInterface|Viewport|AddtoViewport _output_get 0)
  (Widget|SetVisibility _output_get "Collapsed"))

(event Collision|EventActorBeginOverlap
  (params (OtherActor :type Actor%20Object%20Reference))
  (|CallParentFunction OtherActor) ; This node is disabled and will not be called.\nDrag off pins to build functionality.
)

(event EventTick
  (params (DeltaSeconds :type Float%20%28single-precision%29))
  (|CallParentFunction DeltaSeconds) ; This node is disabled and will not be called.\nDrag off pins to build functionality.
)

(fn ConstructionScript
  (|CallParentFunction))

(fn InteractObject
  (params (Item :type EItems%20Enum :default "NewEnumerator8"))
  (bind _overlappingactors (Collision|GetOverlappingActors "/Game/Blueprints/CH_PlayerCharacter.CH_PlayerCharacter_C" :!class /Script/Engine.Actor))
  (bind _defaultsceneroot (Variables|Default|GetDefaultSceneRoot))
  (bind _returnvalue (Transformation|GetWorldLocation _defaultsceneroot))
  (bind _returnvalue_2 (+ "-40.000000,0.000000,10.000000" _returnvalue))
  ;[0.05127 0.05127 0.05127] Get player character
  (if (Utilities|Array|IsEmpty _overlappingactors)
    (Development|PrintString "Closet Lock cannot get player character")
    (return false)
    (else
      (bind _asch_player_character (Utilities|Casting|CastToCH_PlayerCharacter (Utilities|Array|Get(acopy) _overlappingactors)))
      (LocalVariables|SetPlayerCharacter _asch_player_character)
      (if (Variables|Default|GetIsInteracting?)
        ;[0.05127 0.05127 0.05127] Close zoom to lock
        (Variables|Default|SetIsInteracting? false)
        (CallFunction|HideCursor)
        (Widget|SetVisibility (Variables|Default|GetInteractionUI) "Collapsed")
        (Default|DisableZoomCamera (LocalVariables|GetPlayerCharacter))
        (Transformation|SetRelativeLocation (Variables|Default|GetWidget) "0.000000,20.000000,0.000000" false false)
        (return false)
        (else
          ;[0.05127 0.05127 0.05127] Open zoom to lock
          (Transformation|SetRelativeLocation (Variables|Default|GetWidget) "-20.000000,5.000000,0.000000" false false)
          (Default|EnableZoomCamera (LocalVariables|GetPlayerCharacter) _returnvalue_2 (Math|Rotator|FindLookatRotation _returnvalue_2 _returnvalue))
          (Variables|Default|SetIsInteracting? true)
          (Widget|SetVisibility (Variables|Default|GetInteractionUI) "Visible")
          (CallFunction|ShowCursor)
          (return false))))))