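; BP_CabinetDoor is a locked cabinet door that opens when interacted with using a key item.
; InteractObject checks the passed item against one enum entry and, on a match, instantly rotates the door mesh, sets IsOpen and returns true.
; A wrong item returns false, and both outcomes show a WBP_Notification message.
; The door has no closing logic, and interaction does nothing once it is open.
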(event EventBeginPlay
  (|CallParentFunction) ; This node is disabled and will not be called.\nDrag off pins to build functionality.
)

(event Collision|EventActorBeginOverlap
  (params (OtherActor :type Actor%20Object%20Reference))
  (|CallParentFunction OtherActor) ; This node is disabled and will not be called.\nDrag off pins to build functionality.
)

(event EventTick
  (params (DeltaSeconds :type Float%20%28single-precision%29))
  (|CallParentFunction DeltaSeconds) ; This node is disabled and will not be called.\nDrag off pins to build functionality.
)

(fn ConstructionScript
  (|CallParentFunction))

(fn InteractObject
  (params (Item :type EItems%20Enum :default "NewEnumerator8"))
  (if (not (Variables|Default|GetIsOpen?))
    (if (Utilities|Enum|Equal(Enum) Item "NewEnumerator17")
      (Transformation|AddLocalRotation (Variables|Default|GetFinaleCabinetDoor_a) "0.000000,-100.000000, 0" false false)
      (bind _output_get (Variables|Default|SetIsOpen? true))
      ;[0.05127 0.05127 0.05127] Display success notification
      (bind _returnvalue (UserInterface|CreateWidget "/Game/UMG/WBP_Notification.WBP_Notification_C"))
      (Default|SetText _returnvalue "You opened the cabinet with a key!")
      (Default|EventRemoveSelf _returnvalue)
      (UserInterface|Viewport|AddtoViewport _returnvalue 0)
      (return _output_get)
      (else
        ;[0.05127 0.05127 0.05127] Display fail notification
        (bind _returnvalue_2 (UserInterface|CreateWidget "/Game/UMG/WBP_Notification.WBP_Notification_C"))
        (Default|SetText _returnvalue_2 "The cabinet is locked, and use the key to open.")
        (Default|EventRemoveSelf _returnvalue_2)
        (UserInterface|Viewport|AddtoViewport _returnvalue_2 0)
        (return false)))))