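; BP_Postcard is an interactable postcard that toggles a zoomed camera view when the player uses it.
; InteractObject finds the overlapping CH_PlayerCharacter, then enables or disables its zoom camera, aimed at the postcard's root from a fixed world-space offset.
; The Widget component is moved and shrunk while zoomed and reset on exit, with IsInteracting tracking the state.
; The function ignores its Item input and always returns false.
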(event EventBeginPlay
  (|CallParentFunction) ; This node is disabled and will not be called.\nDrag off pins to build functionality.
)

(event Collision|EventActorBeginOverlap
  (params (OtherActor :type Actor%20Object%20Reference))
  (|CallParentFunction OtherActor) ; This node is disabled and will not be called.\nDrag off pins to build functionality.
)

(event EventTick
  (params (DeltaSeconds :type Float%20%28single-precision%29))
  (|CallParentFunction DeltaSeconds) ; This node is disabled and will not be called.\nDrag off pins to build functionality.
)

(fn ConstructionScript
  (|CallParentFunction))

(fn InteractObject
  (params (Item :type EItems%20Enum :default "NewEnumerator8"))
  (bind _overlappingactors (Collision|GetOverlappingActors "/Game/Blueprints/CH_PlayerCharacter.CH_PlayerCharacter_C" :!class /Script/Engine.Actor))
  (bind _defaultsceneroot (Variables|Default|GetDefaultSceneRoot))
  (bind _returnvalue (Transformation|GetWorldLocation _defaultsceneroot))
  (bind _returnvalue_2 (+ "-5.000000,10.000000,25.000000" _returnvalue))
  ;[0.05127 0.05127 0.05127] Get player character
  (if (Utilities|Array|IsEmpty _overlappingactors)
    (Development|PrintString "Postcard cannot get player character")
    (return false)
    (else
      (bind _asch_player_character (Utilities|Casting|CastToCH_PlayerCharacter (Utilities|Array|Get(acopy) _overlappingactors)))
      (LocalVariables|SetPlayerCharacter _asch_player_character)
      (if (Variables|Default|GetIsInteracting?)
        ;[0.05127 0.05127 0.05127] Close zoom to postcard
        (Variables|Default|SetIsInteracting? false)
        (Default|DisableZoomCamera (LocalVariables|GetPlayerCharacter))
        (Transformation|SetRelativeTransform (Variables|Default|GetWidget) (Math|Transform|MakeTransform "0.000000,0.000000,30.000000") false false)
        (return false)
        (else
          ;[0.05127 0.05127 0.05127] Open zoom to postcard
          (Transformation|SetRelativeTransform (Variables|Default|GetWidget) (Math|Transform|MakeTransform "-15.000000,-2.000000,2.000000" "0, 0, 0" "0.500000,0.500000,0.500000") false false)
          (Default|EnableZoomCamera (LocalVariables|GetPlayerCharacter) _returnvalue_2 (Math|Rotator|FindLookatRotation _returnvalue_2 _returnvalue))
          (Variables|Default|SetIsInteracting? true)
          (return false))))))