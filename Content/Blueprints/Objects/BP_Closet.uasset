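; BP_Closet is an interactable cupboard that stays locked behind a passcode, with a chest child actor inside.
; The chest's collider starts disabled, and Tick polls the passcode lock's UI for authentication.
; On success, InteractObject swings both doors open instantly, disables the lock's collider and enables the chest's.
; Opening is one-way, as the closing logic is left unconnected.
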(event Collision|EventActorBeginOverlap
  (params (OtherActor :type Actor%20Object%20Reference))
  (|CallParentFunction OtherActor) ; This node is disabled and will not be called.\nDrag off pins to build functionality.
)

(event EventTick
  (params (DeltaSeconds :type Float%20%28single-precision%29))
  (|CallParentFunction DeltaSeconds)
  (bind _asbp_closet_passcode_lock (Utilities|Casting|CastToBP_ClosetPasscodeLock (Variables|/Script/Engine.ChildActorComponent|GetChildActor (Variables|Default|GetBP_ClosetPasscodeLock))))
  (if (Variables|/Game/UMG/WBP_ClosetPasscodeLock.WBP_ClosetPasscodeLock_C|GetIsAuthenticated? (Variables|/Game/Blueprints/Objects/BP_ClosetPasscodeLock.BP_ClosetPasscodeLock_C|GetInteractionUI _asbp_closet_passcode_lock))
    (CallFunction|InteractObject _asbp_closet_passcode_lock "NewEnumerator2")
    (CallFunction|InteractObject "NewEnumerator2")
    (Variables|/Game/UMG/WBP_ClosetPasscodeLock.WBP_ClosetPasscodeLock_C|SetIsAuthenticated? (Variables|/Game/Blueprints/Objects/BP_ClosetPasscodeLock.BP_ClosetPasscodeLock_C|GetInteractionUI _asbp_closet_passcode_lock) false)))

(event EventBeginPlay
  (|CallParentFunction)
  (bind _asbp_chest (Utilities|Casting|CastToBP_Chest (Variables|/Script/Engine.ChildActorComponent|GetChildActor (Variables|Default|GetBP_Chest))))
  (Default|DisableCollider _asbp_chest))

(fn ConstructionScript
  (|CallParentFunction))

(fn InteractObject
  (params (Item :type EItems%20Enum :default "NewEnumerator8"))
  (if (not (Variables|Default|GetIsOpen?))
    (Transformation|AddLocalRotation (Variables|Default|GetSM_Classic_Cupboard_Door_Left) "0,140.000000, 0" false false)
    (Transformation|AddLocalRotation (Variables|Default|GetSM_Classic_Cupboard_Door_Right) "0,-150.000000, 0" false false)
    (bind _asbp_closet_passcode_lock (Utilities|Casting|CastToBP_ClosetPasscodeLock (Variables|/Script/Engine.ChildActorComponent|GetChildActor (Variables|Default|GetBP_ClosetPasscodeLock))))
    (Default|DisableCollider _asbp_closet_passcode_lock)
    (bind _asbp_chest (Utilities|Casting|CastToBP_Chest (Variables|/Script/Engine.ChildActorComponent|GetChildActor (Variables|Default|GetBP_Chest))))
    (Default|EnableCollider _asbp_chest)
    (Variables|Default|SetIsOpen? true)))

(fn DisableColliders
  (bind _rightboxcollider (Variables|Default|GetRightBoxCollider))
  (bind _leftboxcollider (Variables|Default|GetLeftBoxCollider))
  (Collision|SetCollisionResponsetoChannel _leftboxcollider "ECC_Pawn" "ECR_Ignore")
  (Collision|SetCollisionEnabled _leftboxcollider "NoCollision")
  (Collision|SetCollisionResponsetoChannel _rightboxcollider "ECC_Pawn" "ECR_Ignore")
  (Collision|SetCollisionEnabled _rightboxcollider "NoCollision")
  (Rendering|SetVisibility (Variables|Default|GetWidget) false false))

(fn EnableColliders
  (bind _rightboxcollider (Variables|Default|GetRightBoxCollider))
  (bind _leftboxcollider (Variables|Default|GetLeftBoxCollider))
  (Collision|SetCollisionEnabled _leftboxcollider "QueryOnly")
  (Collision|SetCollisionResponsetoChannel _leftboxcollider "ECC_Pawn" "ECR_Overlap")
  (Collision|SetCollisionEnabled _rightboxcollider "QueryOnly")
  (Collision|SetCollisionResponsetoChannel _rightboxcollider "ECC_Pawn" "ECR_Overlap")
  (Rendering|SetVisibility (Variables|Default|GetWidget) true false))