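; Fridge object with two doors that swing open or shut when interacted with.
; InteractObject flips the IsOpen flag and applies instant local rotations to DoorLeft and DoorRight, with no animation.
; The left door reverses its rotation on closing, while the right door turns the same direction in both branches, so it does not return to its closed position.
; The event graph holds only disabled default events.
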(event EventBeginPlay
  (|CallParentFunction) ; This node is disabled and will not be called.\nDrag off pins to build functionality.
)

(event Collision|EventActorBeginOverlap
  (params (OtherActor :type Actor%20Object%20Reference))
  (|CallParentFunction OtherActor) ; This node is disabled and will not be called.\nDrag off pins to build functionality.
)

(event EventTick
  (params (DeltaSeconds :type Float%20%28single-precision%29))
  (|CallParentFunction DeltaSeconds) ; This node is disabled and will not be called.\nDrag off pins to build functionality.
)

(fn ConstructionScript
  (|CallParentFunction))

(fn InteractObject
  (bind _door_left (Variables|Default|GetDoor_Left))
  (bind _door_right (Variables|Default|GetDoor_Right))
  (if (Variables|Default|GetIsOpen?)
    (Transformation|AddLocalRotation _door_left "0,-130.000000, 0" false false)
    (Transformation|AddLocalRotation _door_right "0,-130.000000, 0" false false)
    (Variables|Default|SetIsOpen? false)
    (else
      (Transformation|AddLocalRotation _door_left "0,130.000000, 0" false false)
      (Transformation|AddLocalRotation _door_right "0,-130.000000, 0" false false)
      (Variables|Default|SetIsOpen? true))))