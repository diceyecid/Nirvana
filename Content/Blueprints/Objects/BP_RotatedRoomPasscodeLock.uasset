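; Interactable keypad lock that sends the player to one of four rotated-room levels depending on the passcode entered.
; Interacting toggles a zoom camera on the lock, shows or hides the cursor and shifts the widget.
; Clickable number meshes append to the passcode string, with a reset button to clear it.
; Enter selects the level by code, saves the player's transform in BP_GameInstance and opens the level; UnlockRoom is empty.
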(event EventBeginPlay
  (|CallParentFunction) ; This node is disabled and will not be called.\nDrag off pins to build functionality.
)

(event Collision|EventActorBeginOverlap
  (params (OtherActor :type Actor%20Object%20Reference))
  (|CallParentFunction OtherActor) ; This node is disabled and will not be called.\nDrag off pins to build functionality.
)

(event EventTick
  (params (DeltaSeconds :type Float%20%28single-precision%29))
  (|CallParentFunction DeltaSeconds) ; This node is disabled and will not be called.\nDrag off pins to build functionality.
)

(event OnClicked(SM_NumberButton_1)
  (params (TouchedComponent :type Primitive%20Component%20Object%20Reference) (ButtonPressed :type Key%20Structure :default "None"))
  (CallFunction|InputPasscode "1")
  (Development|PrintString (Variables|Default|GetPasscode)))

(event OnClicked(SM_NumberButton_8)
  (params (TouchedComponent :type Primitive%20Component%20Object%20Reference) (ButtonPressed :type Key%20Structure :default "None"))
  (CallFunction|InputPasscode "8")
  (Development|PrintString (Variables|Default|GetPasscode)))

(event OnClicked(SM_ResetButton)
  (params (TouchedComponent :type Primitive%20Component%20Object%20Reference) (ButtonPressed :type Key%20Structure :default "None"))
  (CallFunction|ResetPasscode)
  (Development|PrintString (Variables|Default|GetPasscode)))

(event OnClicked(SM_EnterButton)
  (params (TouchedComponent :type Primitive%20Component%20Object%20Reference) (ButtonPressed :type Key%20Structure :default "None"))
  (CallFunction|EnterPasscode))

(event OnClicked(SM_NumberButton_6)
  (params (TouchedComponent :type Primitive%20Component%20Object%20Reference) (ButtonPressed :type Key%20Structure :default "None"))
  (CallFunction|InputPasscode "6")
  (Development|PrintString (Variables|Default|GetPasscode)))

(event OnClicked(SM_NumberButton_2)
  (params (TouchedComponent :type Primitive%20Component%20Object%20Reference) (ButtonPressed :type Key%20Structure :default "None"))
  (CallFunction|InputPasscode "2")
  (Development|PrintString (Variables|Default|GetPasscode)))

(event OnClicked(SM_NumberButton_3)
  (params (TouchedComponent :type Primitive%20Component%20Object%20Reference) (ButtonPressed :type Key%20Structure :default "None"))
  (CallFunction|InputPasscode "3")
  (Development|PrintString (Variables|Default|GetPasscode)))

(event OnClicked(SM_NumberButton_7)
  (params (TouchedComponent :type Primitive%20Component%20Object%20Reference) (ButtonPressed :type Key%20Structure :default "None"))
  (CallFunction|InputPasscode "7")
  (Development|PrintString (Variables|Default|GetPasscode)))

(event OnClicked(SM_NumberButton_4)
  (params (TouchedComponent :type Primitive%20Component%20Object%20Reference) (ButtonPressed :type Key%20Structure :default "None"))
  (CallFunction|InputPasscode "4")
  (Development|PrintString (Variables|Default|GetPasscode)))

(event OnClicked(SM_NumberButton_9)
  (params (TouchedComponent :type Primitive%20Component%20Object%20Reference) (ButtonPressed :type Key%20Structure :default "None"))
  (CallFunction|InputPasscode "9")
  (Development|PrintString (Variables|Default|GetPasscode)))

(event OnClicked(SM_NumberButton_5)
  (params (TouchedComponent :type Primitive%20Component%20Object%20Reference) (ButtonPressed :type Key%20Structure :default "None"))
  (CallFunction|InputPasscode "5")
  (Development|PrintString (Variables|Default|GetPasscode)))

(fn ConstructionScript
  (|CallParentFunction))

(fn InteractObject
  (params (Item :type EItems%20Enum :default "NewEnumerator8"))
  (bind _overlappingactors (Collision|GetOverlappingActors "/Game/Blueprints/CH_PlayerCharacter.CH_PlayerCharacter_C" :!class /Script/Engine.Actor))
  (bind _defaultsceneroot (Variables|Default|GetDefaultSceneRoot))
  (bind _returnvalue (Transformation|GetWorldLocation _defaultsceneroot))
  (bind _returnvalue_2 (+ "-50.000000,0.000000,0.000000" _returnvalue))
  ;[0.05127 0.05127 0.05127] Get player character
  (if (Utilities|Array|IsEmpty _overlappingactors)
    (Development|PrintString "Postcard cannot get player character")
    (return false)
    (else
      (bind _asch_player_character (Utilities|Casting|CastToCH_PlayerCharacter (Utilities|Array|Get(acopy) _overlappingactors)))
      (LocalVariables|SetPlayerCharacter _asch_player_character)
      (if (Variables|Default|GetIsInteracting?)
        ;[0.05127 0.05127 0.05127] Close zoom to lock
        (Variables|Default|SetIsInteracting? false)
        (CallFunction|HideCursor)
        (Default|DisableZoomCamera (LocalVariables|GetPlayerCharacter))
        (Transformation|SetRelativeLocation (Variables|Default|GetWidget) "0.000000,20.000000,-10.000000" false false)
        (return false)
        (else
          ;[0.05127 0.05127 0.05127] Open zoom to lock
          (Transformation|SetRelativeLocation (Variables|Default|GetWidget) "-35.000000,5.000000,-10.000000" false false)
          (Default|EnableZoomCamera (LocalVariables|GetPlayerCharacter) _returnvalue_2 (Math|Rotator|FindLookatRotation _returnvalue_2 _returnvalue))
          (Variables|Default|SetIsInteracting? true)
          (CallFunction|ShowCursor)
          (return false))))))

(fn UnlockRoom)

(fn ResetPasscode
  (Variables|Default|SetPasscode "")
  (return))

(fn InputPasscode
  (params (Number :type String))
  (Variables|Default|SetPasscode (Utilities|String|Append (Variables|Default|GetPasscode) Number))
  (return))

(fn EnterPasscode
  (bind _returnvalue (Game|GetPlayerCharacter 0))
  (switch string (Variables|Default|GetPasscode)
    (:321587
      (LocalVariables|SetRotatedRoomLevel "/Game/Levels/Rotate_0.Rotate_0"))
    (:254789
      (LocalVariables|SetRotatedRoomLevel "/Game/Levels/Rotate90.Rotate90"))
    (:965214
      (LocalVariables|SetRotatedRoomLevel "/Game/Levels/Rotate_180.Rotate_180"))
    (:357852
      (LocalVariables|SetRotatedRoomLevel "/Game/Levels/Rotate_270.Rotate_270")))
  (CallFunction|HideCursor)
  (bind _asbp_game_instance (Utilities|Casting|CastToBP_GameInstance (Game|GetGameInstance)))
  (Variables|/Game/Blueprints/BP_GameInstance.BP_GameInstance_C|SetPlayerHouseLocation _asbp_game_instance (Transformation|GetActorLocation _returnvalue))
  (Variables|/Game/Blueprints/BP_GameInstance.BP_GameInstance_C|SetPlayerHouseRotation _asbp_game_instance (Transformation|GetActorRotation _returnvalue))
  (Game|OpenLevel(byObjectReference) (LocalVariables|GetRotatedRoomLevel))
  (return))