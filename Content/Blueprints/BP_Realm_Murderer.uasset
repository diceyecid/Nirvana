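; BP_Realm_Murderer is an AI-driven pawn that chases the player in the Realm game and ends the game on catching them.
; Every Tick issues AIMoveTo toward the player character; when the move succeeds and the two overlap, it calls GameOver.
; GameOver clears IsBeingControlled on CH_RealmCharacter, shows WBP_RealmGameOver and switches to UI-only input with the mouse cursor visible.
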(event EventBeginPlay)

(event Collision|EventActorBeginOverlap
  (params (OtherActor :type Actor%20Object%20Reference)))

(event EventTick
  (params (DeltaSeconds :type Float%20%28single-precision%29))
  (bind _returnvalue (Game|GetPlayerCharacter 0))
  (AI|AIMoveTo self "0, 0, 0" _returnvalue 5.0 false
    (:then
      (if (Collision|IsOverlappingActor _returnvalue self :!class /Script/Engine.Actor)
        (CallFunction|GameOver)))))

(fn ConstructionScript)

(fn GameOver
  (bind _returnvalue (Game|GetPlayerController 0))
  (bind _asch_realm_character (Utilities|Casting|CastToCH_RealmCharacter (Game|GetPlayerCharacter 0)))
  (Variables|/Game/Blueprints/CH_RealmCharacter.CH_RealmCharacter_C|SetIsBeingControlled? _asch_realm_character false)
  (bind _returnvalue_2 (UserInterface|CreateWidget "/Game/UMG/WBP_RealmGameOver.WBP_RealmGameOver_C" _returnvalue))
  (UserInterface|Viewport|AddtoViewport _returnvalue_2 0)
  (Variables|/Script/Engine.PlayerController|SetbShowMouseCursor _returnvalue true)
  (Variables|/Script/Engine.PlayerController|SetbEnableClickEvents _returnvalue true)
  (Input|SetInputModeUIOnly _returnvalue _returnvalue_2 "DoNotLock"))