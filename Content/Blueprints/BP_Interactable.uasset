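; Base interactable actor that shows a key prompt when the player character is in range.
; BeginPlay sets the WBP_PopUp widget text by subclass: "E" for BP_Prop children, "F" for BP_Object children.
; Each Tick polls for overlapping CH_PlayerCharacter actors, showing the widget and turning it toward the camera during overlap, and hiding it otherwise.
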(event EventBeginPlay
  (CallFunction|SetPopUpText))

(event EventTick
  (params (DeltaSeconds :type Float%20%28single-precision%29))
  (CallFunction|ManagePopUp))

(fn ConstructionScript)

(fn SetPopUpText
  (bind _aswbp_pop_up (Utilities|Casting|CastToWBP_PopUp (UserInterface|GetUserWidgetObject (Variables|Default|GetWidget))))
  ;[0.05127 0.05127 0.05127] Set pop up text for prop
  (if (Utilities|ClassIsChildOf (Utilities|GetClass self) "/Game/Blueprints/Props/BP_Prop.BP_Prop_C")
    (Default|SetText _aswbp_pop_up "E")
    (return)
    (else
      ;[0.05127 0.05127 0.05127] Set pop up text for interactable object
      (if (Utilities|ClassIsChildOf (Utilities|GetClass self) "/Game/Blueprints/Objects/BP_Object.BP_Object_C")
        (Default|SetText _aswbp_pop_up "F")
        (return)))))

(fn ManagePopUp
  (bind _widget (Variables|Default|GetWidget))
  (if (Utilities|Array|IsNotEmpty (Collision|GetOverlappingActors "/Game/Blueprints/CH_PlayerCharacter.CH_PlayerCharacter_C" :!class /Script/Engine.Actor))
    ;[0.05127 0.05127 0.05127] Within interactable range, turn on pop up and rotate to face camera
    (Transformation|SetWorldRotation _widget (Math|Rotator|FindLookatRotation (Transformation|GetWorldLocation _widget) (Camera|GetCameraLocation (Game|GetPlayerCameraManager 0))) false false)
    (Rendering|SetVisibility (Variables|Default|GetWidget) true false)
    (else
      ;[0.05127 0.05127 0.05127] Out of range, turn off pop up
      (Rendering|SetVisibility (Variables|Default|GetWidget) false false)))
  (return))